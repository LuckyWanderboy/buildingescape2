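; BP_StudentSpawner spawns AI students that represent chatters received through a message interface event.
; Each event stores the chatter data and spawns one of two random pawn types at a nearby navigable point, with randomized height.
; It then applies name and color to the widget, logo to the head, and color to outfit slots via dynamic materials.
; Tab debug-spawns students; female ones occasionally show Toast.
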(event Custom|Spawn%20Student
  (bind _randomlocation (Class|NavigationSystemV1|GetRandomLocationinNavigableRadius (Transformation|GetActorLocation self) 3e+02 0 0))
  (bind _returnvalue (AI|SpawnAIFromClass (Utilities|Array|Get(acopy) (Variables|Default|GetStudentPawnTypess) (Math|Random|RandomIntegerinRange 0 1)) 0 _randomlocation "0, 0, 0" true 0))
  (bind _output_get (Variables|Default|SetOut%20ofSpawn _returnvalue))
  (bind _ascubface (Utilities|Casting|CastTocubface _output_get))
  (bind _output_get_2 (Variables|Default|SetAs%20Cubface _ascubface))
  (Transformation|SetActorRelativeScale3D _output_get_2 (Math|Vector|MakeVector 1.0 1.0 (Math|Random|RandomFloatinRange 1.0 1.3)))
  (bind _ascubfacefemale (Utilities|Casting|CastTocubfacefemale (Variables|Default|GetOut%20ofSpawn)))
  (Development|SetHiddeninGame (Variables|/Game/Pawns/Students/Female/cubfacefemale.cubfacefemale_C|Gettoast _ascubfacefemale) (Math|Random|RandomBoolwithWeight 0.95) false))

(event EventMessageInterface
  (params (chatter_name :type String) (chatter_message :type Text) (chatter_logo :type Texture%202D%20Object%20Reference) (chatter_color :type Color%20Structure))
  (|SetAllParameters chatter_name chatter_message chatter_logo chatter_color)
  (CallFunction|SpawnStudent)
  (Utilities|SetChatterDisplayName)
  (Utilities|SetLogo)
  (CallFunction|SetOutfitColor)
  (CallFunction|SetOutfitColor 4)
  (CallFunction|SetOutfitColor 5))

(event Input|KeyboardEvents|DebugKeyTab
  (params (Key :type Key%20Structure :default "None") (ActionValue :type Input%20Action%20Value%20Structure))
  (:Pressed
    (bind _randomlocation (Class|NavigationSystemV1|GetRandomLocationinNavigableRadius (Transformation|GetActorLocation self) 3e+02 0 0))
    (bind _returnvalue (AI|SpawnAIFromClass (Utilities|Array|Get(acopy) (Variables|Default|GetStudentPawnTypess) (Math|Random|RandomIntegerinRange 0 1)) 0 _randomlocation "0, 0, 0" true 0))
    (bind _output_get (Variables|Default|SetOut%20ofSpawn _returnvalue))
    (bind _ascubface (Utilities|Casting|CastTocubface _output_get))
    (bind _output_get_2 (Variables|Default|SetAs%20Cubface _ascubface))
    (Transformation|SetActorRelativeScale3D _output_get_2 (Math|Vector|MakeVector 1.0 1.0 (Math|Random|RandomFloatinRange 1.0 1.3)))
    (bind _ascubfacefemale (Utilities|Casting|CastTocubfacefemale (Variables|Default|GetOut%20ofSpawn)))
    (Development|SetHiddeninGame (Variables|/Game/Pawns/Students/Female/cubfacefemale.cubfacefemale_C|Gettoast _ascubfacefemale) (Math|Random|RandomBoolwithWeight 0.95) false)))

(fn ConstructionScript)

(fn SetOutfitColor
  (params (ElementIndex :type Integer))
  (bind _returnvalue (Rendering|Material|CreateDynamicMaterialInstance (Variables|/Script/Engine.Character|GetMesh (Variables|Default|GetAs%20Cubface)) ElementIndex "/Game/Pawns/Students/Male/tpose/materials/mii_school_m_shoes.mii_school_m_shoes" "None" :!class /Script/Engine.PrimitiveComponent))
  (Rendering|Material|SetVectorParameterValue _returnvalue "color" (Math|Conversions|ToLinearColor(Color) (Variables|Default|GetChatter%20Color)) :!class /Script/Engine.MaterialInstanceDynamic))