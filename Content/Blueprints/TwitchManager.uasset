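; Twitch manager that lets chat viewers affect the game through chat commands.
; On BeginPlay it logs in, opens the chat feed and registers launch, chair, b and attack commands; plain chat and cheer handlers are empty.
; Chair and ball commands spawn actors at typed XYZ coordinates, tinting balls with the sender's color.
; Launch, attack and ball spawns broadcast through BPI_twitcommand to actors, with ball spawns also reaching widgets.
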(event Custom|ChatEvent
  (params (TwitchMessage :type Twitch%20Message%20Structure)))

(event Custom|CheerEvent
  (params (TwitchCheer :type Twitch%20Cheer%20Structure)))

(event Custom|Spawn%20Chair
  (params (Parameters :type Array%20of%20Strings) (Sender :type Twitch%20Message%20Author%20Structure))
  (Audio|PlaySound2D "/Engine/VREditor/Sounds/UI/Dockable_Window_Drop.Dockable_Window_Drop" 1.0 1.0 0.0 0 0)
  (bind _chair_drop_vector (CallFunction|GetSpawnVector Parameters Parameters Parameters))
  (Game|SpawnActorfromClass "/Game/Blueprints/Chair_kun.Chair_kun_C" (Math|Transform|MakeTransform _chair_drop_vector "0, 0, 0" "1.000000,1.000000,1.000000") "Undefined" "MultiplyWithRoot" 0 0))

(event Custom|TwitchCommands
  (Utilities|FlowControl|Sequence
    (:then_0
      (CallFunction|NewTwitchCommand (Utilities|Struct|MakeTwitchCommand "launch" "" 0 false) (delegate Custom|ChairJump)))
    (:then_1
      (CallFunction|NewTwitchCommand (Utilities|Struct|MakeTwitchCommand "chair" "" (Utilities|GetFvectorParameters) false) (delegate Custom|Spawn%20Chair)))
    (:then_2
      ;[1 1 1] Spawn Ball
      (CallFunction|NewTwitchCommand (Utilities|Struct|MakeTwitchCommand "b" "" (Utilities|GetFvectorParameters) false) (delegate Custom|SpawnBall)))
    (:then_3
      (CallFunction|NewTwitchCommand (Utilities|Struct|MakeTwitchCommand "attack" "" 0 false) (delegate Custom|attack)))))

(event Custom|SpawnBall
  (params (Parameters :type Array%20of%20Strings) (Sender :type Twitch%20Message%20Author%20Structure))
  ;[1 1 1] Spawn Ball
  (Variables|Default|SetSpawner_name (.displayname Sender))
  (CallFunction|GetColorVectorCorrect (.r (.color Sender)) (.g (.color Sender)) (.b (.color Sender)))
  (bind _chair_drop_vector (CallFunction|GetSpawnVector Parameters Parameters Parameters))
  (bind _returnvalue (Game|SpawnActorfromClass "/Game/Blueprints/Ball_kun.Ball_kun_C" (Math|Transform|MakeTransform _chair_drop_vector "0, 0, 0" "1.000000,1.000000,1.000000") "Undefined" "MultiplyWithRoot" 0 0))
  (Rendering|Material|SetVectorParameterValueonMaterials (Variables|/Game/Blueprints/Ball_kun.Ball_kun_C|GetSphere _returnvalue) "Color" (Variables|Default|Getcolor%20vector))
  (bind _outactors (Actor|GetAllActorswithInterface "/Game/Blueprints/BPI_twitcommand.BPI_twitcommand_C"))
  (Class|BPITwitcommand|SpawnInterface(Message) _outactors (Variables|Default|Getchair%20drop%20vector) (Variables|Default|GetSpawner_name))
  (bind _foundwidgets (Class|WidgetBlueprintLibrary|GetAllWidgetswithInterface "/Game/Blueprints/BPI_twitcommand.BPI_twitcommand_C" false))
  (Class|BPITwitcommand|SpawnInterface(Message) _foundwidgets (Variables|Default|Getchair%20drop%20vector) (Variables|Default|GetSpawner_name))
  (Development|PrintString (Utilities|String|ToString(Vector) (Variables|Default|Getcolor%20vector))))

(event Custom|ChairJump
  (params (Parameters :type Array%20of%20Strings) (Sender :type Twitch%20Message%20Author%20Structure))
  (bind _outactors (Actor|GetAllActorswithInterface "/Game/Blueprints/BPI_twitcommand.BPI_twitcommand_C"))
  (Class|BPITwitcommand|BpiFnOncommand(Message) _outactors))

(event Custom|attack
  (params (Parameters :type Array%20of%20Strings) (Sender :type Twitch%20Message%20Author%20Structure))
  (bind _outactors (Actor|GetAllActorswithInterface "/Game/Blueprints/BPI_twitcommand.BPI_twitcommand_C"))
  (Class|BPITwitcommand|BpiFnOncommand(Message) _outactors (.displayname Sender)))

(fn ConstructionScript)

(fn NewTwitchCommand
  (params (Command :type Twitch%20Command%20Structure) (Binding :type Delegate))
  (Class|TwitchPluginBPLibrary|CreateTwitchCommand (Variables|Default|GetTwitch%20Chat) (Utilities|Struct|MakeTwitchCommandBinding Command Binding)))

(fn GetSpawnVector
  (params (Array :type Array%20of%20Strings) (Array2 :type Array%20of%20Strings) (Array3 :type Array%20of%20Strings))
  (bind _chair_drop_vector (Variables|Default|Getchair%20drop%20vector))
  (Class|KismetMathLibrary|VectorSet _chair_drop_vector (Math|Conversions|ToFloat(Integer) (Utilities|Array|Get(acopy) Array2)) (Math|Conversions|ToFloat(Integer) (Utilities|Array|Get(acopy) Array 1)) (Math|Conversions|ToFloat(Integer) (Utilities|Array|Get(acopy) Array3 2)))
  (return _chair_drop_vector))

(fn GetColorVector
  (params (A :type Byte) (A2 :type Byte) (A3 :type Byte))
  (Class|KismetMathLibrary|VectorSet (Variables|Default|Getcolor%20vector) (Math|Conversions|ToFloat(Byte) (/ A3 255)) (Math|Conversions|ToFloat(Byte) (/ A2 255)) (Math|Conversions|ToFloat(Byte) (/ A 255))))

(fn NewComand
  (Class|TwitchPluginBPLibrary|CreateTwitchCommand (Variables|Default|GetTwitch%20Chat) (Utilities|Struct|MakeTwitchCommandBinding (Utilities|Struct|MakeTwitchCommand "" "" 0 false) "(null).None")))

(fn GetColorVectorCorrect
  (params (InByte :type Byte) (InByte2 :type Byte) (InByte3 :type Byte))
  (Class|KismetMathLibrary|VectorSet (Variables|Default|Getcolor%20vector) (/ (Math|Conversions|ToFloat(Byte) InByte) 255.0) (/ (Math|Conversions|ToFloat(Byte) InByte2) 255.0) (/ (Math|Conversions|ToFloat(Byte) InByte3) 255.0)))

(event EventBeginPlay
  (bind _credentials (|PerformLocalTwitchLogin)
    (:OnSuccess
      (return _credentials))))

(fn SpawnInterface
  (params (spawn_location :type Vector :default "0, 0, 0") (spawn_name :type String))
  (return))