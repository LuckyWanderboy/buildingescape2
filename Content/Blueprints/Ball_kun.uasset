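; Named ball actor that represents a spawned character with its own logo and floating name, and can be launched by command to attack.
; A spawn interface event fills the name widget and a dynamic logo material on first call, and destroys the ball if its name is sent again.
; A command matching its name applies a fixed impulse to the sphere.
; Overlapping the player pawn prints an attack message and triggers fire and explosion sound.
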(event OnComponentBeginOverlap(Sphere1)
  (params (OverlappedComponent :type Primitive%20Component%20Object%20Reference) (OtherActor :type Actor%20Object%20Reference) (OtherComp :type Primitive%20Component%20Object%20Reference) (OtherBodyIndex :type Integer) (bFromSweep :type Boolean) (SweepResult :type Hit%20Result%20Structure%20%28by%20ref%29))
  (if (== OtherActor (Game|Player|GetPlayerPawn 0))
    (Development|PrintString (Utilities|String|Append (Variables|Default|Getcharacter%20name) " Attacked " (Utilities|GetDisplayName OtherActor)))
    (Effects|SpawnEmitterAttached "/Game/StarterContent/Particles/P_Fire.P_Fire" (Variables|Default|GetSphere) "None")
    (Audio|PlaySound2D "/Game/StarterContent/Audio/Explosion01.Explosion01" 1.0 1.0 0.0 0 0)))

(event EventSpawnInterface
  (params (spawn_location :type Vector :default "0, 0, 0") (spawn_name :type String) (spawn_logo :type Texture%202D%20Object%20Reference) (spawn_color :type Color%20Structure))
  (Variables|Default|SetSpawn%20Color spawn_color)
  (if (Utilities|Array|IsEmpty (Variables|Default|Getcharacter%20name))
    (Variables|Default|Setcharacter%20name spawn_name)
    (bind _aswid_name_display (Utilities|Casting|CastToWID_Name_Display (UserInterface|GetUserWidgetObject (Variables|Default|GetWidget))))
    (Variables|/Game/Blueprints/WID_Name_Display.WID_Name_Display_C|Setspawn_display_text _aswid_name_display (Variables|Default|Getcharacter%20name))
    (bind _returnvalue (Rendering|Material|CreateDynamicMaterialInstance (Variables|Default|GetSphere) 0 "/Game/Blueprints/Logo.Logo" "None" :!class /Script/Engine.PrimitiveComponent))
    (Rendering|Material|SetTextureParameterValue _returnvalue "Logo" spawn_logo)
    (Variables|/Game/Blueprints/WID_Name_Display.WID_Name_Display_C|Setspawn_diplay_color _aswid_name_display (Variables|Default|GetSpawn%20Color))
    (elif (Utilities|Enum|Equal(Enum) spawn_name (Variables|Default|Getcharacter%20name))
      (Actor|DestroyActor))))

(event EventBpiFnOncommand
  (params (command_name :type String))
  (bind _character_name (Variables|Default|Getcharacter%20name))
  (if (Utilities|Enum|Equal(Enum) command_name _character_name)
    (Development|PrintString (Utilities|String|Append "attacked with " _character_name))
    (Physics|AddImpulse (Variables|Default|GetSphere) "100000.000000,0.000000,10000.000000" "None" false)))

(fn ConstructionScript)

(fn SetLogo
  (params (Value :type Texture%20Object%20Reference))
  (bind _returnvalue (Rendering|Material|CreateDynamicMaterialInstance (Variables|Default|GetSphere) 0 "/Game/Blueprints/Logo.Logo" "None" :!class /Script/Engine.PrimitiveComponent))
  (Rendering|Material|SetTextureParameterValue _returnvalue "Logo" Value))