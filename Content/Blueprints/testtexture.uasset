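; Test actor Blueprint that applies a logo texture and a color to its meshes when its SpawnInterface event fires.
; The event prints a debug message, creates a dynamic material instance on PlaneTest and sets the incoming texture as its Logo parameter.
; It stores the incoming color, divides its RGB bytes by 255 and writes the result to the Color vector parameter on Cube's materials.
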(event EventSpawnInterface
  (params (spawn_location :type Vector :default "0, 0, 0") (spawn_name :type String) (spawn_logo :type Texture%202D%20Object%20Reference) (spawn_color :type Color%20Structure))
  (Development|PrintText "logo set")
  (bind _returnvalue (Rendering|Material|CreateDynamicMaterialInstance (Variables|Default|GetPlane_test) 0 0 "None" :!class /Script/Engine.PrimitiveComponent))
  (Rendering|Material|SetTextureParameterValue _returnvalue "Logo" spawn_logo)
  (bind _output_get (Variables|Default|SetSpawn%20Color spawn_color))
  (Rendering|Material|SetVectorParameterValueonMaterials (Variables|Default|GetCube) "Color" (Math|Vector|MakeVector (/ (Math|Conversions|ToFloat(Byte) (.r _output_get)) 255.0) (/ (Math|Conversions|ToFloat(Byte) (.g _output_get)) 255.0) (/ (Math|Conversions|ToFloat(Byte) (.b _output_get)) 255.0))))

(fn ConstructionScript)